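; BP_AwesomePlayerController is a player controller that lets the player toggle the inventory and equipment screen.
; On BeginPlay it creates WBP_InventoryAndEquipment, adds it to the viewport and hides it.
; The I key drives a FlipFlop that shows or hides the widget, toggles the mouse cursor, and switches between Game and UI input focused on the widget and game-only input.
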(event `self.ReceiveBeginPlay`
  (bind _returnvalue (`|CreateWidget` "/Game/Blueprints/UI/WBP_InventoryAndEquipment.WBP_InventoryAndEquipment_C"))
  (bind _output_get (set `self.Interface` _returnvalue))
  (`UserWidget.AddToViewport` _output_get 0)
  (`Widget.SetVisibility` (`self.Interface`) "Hidden"))

(event `Key|I`
  (params (Key :type "Key Structure"))
  (bind _returnvalue (`GameplayStatics.GetPlayerController` 0))
  (:`Pressed`
    (bind _isa (`/Engine/EditorBlueprintResources/StandardMacros.FlipFlop`)
      (:`A`
        (`WidgetBlueprintLibrary.SetInputMode_GameAndUIEx` _returnvalue (`self.Interface`)))
      (:`B`
        (`WidgetBlueprintLibrary.SetInputMode_GameOnly` _returnvalue)))
    (`Widget.SetVisibility` (`self.Interface`) (select `bool` _isa :`false` "Hidden" :`true` "Visible" :!type "ESlateVisibility Enum"))
    (set `PlayerController.bShowMouseCursor` _isa (`GameplayStatics.GetPlayerController` 0))))

(fn `UserConstructionScript`)